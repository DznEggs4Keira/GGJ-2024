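; Game mode for local multiplayer that creates players and spawns their kobold characters.
; On BeginPlay it gathers PlayerStarts and, for each array index matching a numeric PlayerStartTag, creates a local player possessing a BP_InputReciever spawned at that index's start, which need not be the tagged one.
; SpawnPlayer, not called here, spawns a Small, Tall or Wide kobold by player index at the given receiver's transform and possesses it.
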(event EventBeginPlay
  (CallFunction|GetPlayerStartPoints)
  (CallFunction|SpawnInputrReceivers))

(event EventTick
  (params (DeltaSeconds :type Float%20%28single-precision%29)))

(fn ConstructionScript)

(fn GetPlayerStartPoints
  (bind _outactors (Actor|GetAllActorsOfClass "/Script/Engine.PlayerStart"))
  (Variables|Default|SetPlayerStartArray _outactors))

(fn SpawnInputrReceivers
  (for (_ _array_index) (Variables|Default|GetPlayerStartArray)
    (LocalVariables|SetIndex _array_index)
    (for _array_element (Variables|Default|GetPlayerStartArray)
      (if (== (LocalVariables|GetIndex) (CallFunction|NametoInt _array_element))
        (Class|GameplayStatics|CreatePlayer -1)
        (bind _returnvalue (Game|SpawnActorfromClass "/Game/Blueprints/Multiplayer/BP_InputReciever.BP_InputReciever_C" (Transformation|GetActorTransform (Utilities|Array|Get(acopy) (Variables|Default|GetPlayerStartArray) (LocalVariables|GetIndex))) "Undefined" "MultiplyWithRoot" 0 (LocalVariables|GetIndex) 0))
        (Utilities|Array|AddUnique (Variables|Default|GetPlayerInputReceiverArray) _returnvalue)
        (Pawn|Possess (Game|GetPlayerController (LocalVariables|GetIndex)) _returnvalue)
        (Utilities|Array|AddUnique (Variables|Default|GetPlayerControllerArray) (Game|GetPlayerController (LocalVariables|GetIndex)))))))

(fn NametoInt
  (params (self2 :type Player%20Start%20Object%20Reference))
  (return (Math|Conversions|ToInteger(Byte) (Utilities|String|ToString(Name) (Variables|/Script/Engine.PlayerStart|GetPlayerStartTag self2)))))

(fn SpawnPlayer
  (params (CurrentPlayerIndex :type Integer) (InputReceiver :type BP%20Input%20Reciever%20Object%20Reference))
  (switch int CurrentPlayerIndex
    (:0
      (bind _returnvalue (Game|SpawnActorfromClass "/Game/Blueprints/BP_Kobold_Small.BP_Kobold_Small_C" (Transformation|GetActorTransform InputReceiver) "Undefined" "MultiplyWithRoot" 0 CurrentPlayerIndex 0))
      (Pawn|Possess (Game|GetPlayerController CurrentPlayerIndex) _returnvalue))
    (:1
      (bind _returnvalue_2 (Game|SpawnActorfromClass "/Game/Blueprints/BP_Kobold_Tall.BP_Kobold_Tall_C" (Transformation|GetActorTransform InputReceiver) "Undefined" "MultiplyWithRoot" 0 CurrentPlayerIndex 0))
      (Pawn|Possess (Game|GetPlayerController CurrentPlayerIndex) _returnvalue_2))
    (:2
      (bind _returnvalue_3 (Game|SpawnActorfromClass "/Game/Blueprints/BP_Kobold_Wide.BP_Kobold_Wide_C" (Transformation|GetActorTransform InputReceiver) "Undefined" "MultiplyWithRoot" 0 CurrentPlayerIndex 0))
      (Pawn|Possess (Game|GetPlayerController CurrentPlayerIndex) _returnvalue_3)))
  (return false))