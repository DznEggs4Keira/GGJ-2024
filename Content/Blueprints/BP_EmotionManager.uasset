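; BP_EmotionManager is a component for BP_KoboldMain that drives the kobold's face sprite, currently as a temporary random-cycle test.
; On BeginPlay it casts its owner and pools the owner's emotion faces and base faces into one array.
; A looping delay then sets a random sprite from that pool every few seconds, independent of any emotional state.
; Voice references for each emotion are present but unused, and Tick is empty.
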(event EventBeginPlay
  (bind _asbp_kobold_main (Utilities|Casting|CastToBP_KoboldMain (Components|GetOwner)))
  (Variables|Default|SetAs%20BP%20Kobold%20Main _asbp_kobold_main)
  ;[1 0 0] Here you can find all the faces
  (Variables|Default|SetFaceComponent (Variables|/Game/Blueprints/BP_KoboldMain.BP_KoboldMain_C|GetFace (Variables|Default|GetAs%20BP%20Kobold%20Main)))
  (bind _output_get (Variables|Default|SetTEMPAllFaces (Utilities|Array|MakeArray (Variables|/Game/Blueprints/BP_KoboldMain.BP_KoboldMain_C|GetFrustratedFace (Variables|Default|GetAs%20BP%20Kobold%20Main)) (Variables|/Game/Blueprints/BP_KoboldMain.BP_KoboldMain_C|GetDrunkFace (Variables|Default|GetAs%20BP%20Kobold%20Main)) (Variables|/Game/Blueprints/BP_KoboldMain.BP_KoboldMain_C|GetDrinkingFace (Variables|Default|GetAs%20BP%20Kobold%20Main)) (Variables|/Game/Blueprints/BP_KoboldMain.BP_KoboldMain_C|GetGuiltyFace (Variables|Default|GetAs%20BP%20Kobold%20Main)) (Variables|/Game/Blueprints/BP_KoboldMain.BP_KoboldMain_C|GetHappyFace (Variables|Default|GetAs%20BP%20Kobold%20Main)) (Variables|/Game/Blueprints/BP_KoboldMain.BP_KoboldMain_C|GetTippingFace (Variables|Default|GetAs%20BP%20Kobold%20Main)) (Variables|/Game/Blueprints/BP_KoboldMain.BP_KoboldMain_C|GetSpottedFace (Variables|Default|GetAs%20BP%20Kobold%20Main)))))
  (Utilities|Array|AppendArray _output_get (Variables|/Game/Blueprints/BP_KoboldMain.BP_KoboldMain_C|GetBaseFaces (Variables|Default|GetAs%20BP%20Kobold%20Main)))
  ;[1 1 1] TempCycle test
  (Rendering|Components|Sprite|SetSprite (Variables|Default|GetFaceComponent) (.OutItem (Utilities|Array|Random (Variables|Default|GetTEMPAllFaces))) :!label _label)
  (Utilities|FlowControl|Delay (Math|Random|RandomFloatinRange 2.0 5.0))
  (goto _label))

(event EventTick
  (params (DeltaSeconds :type Float%20%28single-precision%29)))