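; BP_ConversationIndicatorBartender is a floating coin indicator for the bartender that shows how many coins are still needed.
; On BeginPlay it sets that count text from the BP_VictoryTrigger's picked-up coins, then reveals and scales up the coin.
; A self-restarting Bounce timeline drifts the coin between random X/Z offsets around its original position with a slight wobble.
; DestroyConversation reverses the scale timeline, then destroys the actor.
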(event EventBeginPlay
  (Rendering|Components|TextRender|SetText)
  (bind _output_get (Variables|Default|SetRelativeT (Transformation|GetRelativeTransform (Variables|Default|GetSM_Coin))))
  (Variables|Default|SetCurrentVec3 (.Location (Math|Transform|BreakTransform _output_get)))
  (Components|Timeline|SetPlayRate (Variables|Default|GetBounce) (/ 1.0 2.0))
  (Utilities|FlowControl|Sequence
    (:then_0
      (Components|Timeline|SetPlayRate (Variables|Default|GetScaleUp) (/ 1.0 1.0))
      (Transformation|SetRelativeScale3D (Variables|Default|GetSM_Coin) "0, 0, 0")
      (Development|SetHiddeninGame (Variables|Default|GetCoinIndicator) false false)
      (bind _lerp (Timeline|ScaleUp PlayFromStart)
        (:Update
          (Transformation|SetRelativeScale3D (Variables|Default|GetSM_Coin) (* _lerp (.Scale (Math|Transform|BreakTransform (Variables|Default|GetRelativeT))))))
        (:Finished
          (if (Variables|Default|GetWIllDestroy)
            (Actor|DestroyActor)))))
    (:then_1
      (Variables|Default|SetRandomVec3 (+ (* (Math|Vector|MakeVector (CallFunction|RandomFloat) 0.0 (CallFunction|RandomFloat)) 1e+01) (.Location (Math|Transform|BreakTransform (Variables|Default|GetRelativeT)))) :!label _label)
      (bind (_direction _rotation _bounce) (Timeline|Bounce PlayFromStart)
        (:Update
          (Transformation|SetRelativeLocationAndRotation (Variables|Default|GetSM_Coin) (Math|Vector|Lerp(Vector) (Variables|Default|GetCurrentVec3) (Variables|Default|GetRandomVec3) _bounce) (Math|Rotator|CombineRotators (Math|Rotator|MakeRotator (* _rotation 1e+01) (* _rotation 5.0) 0.0) (.Rotation (Math|Transform|BreakTransform (Variables|Default|GetRelativeT)))) false false))
        (:Finished
          (Variables|Default|SetCurrentVec3 (Variables|Default|GetRandomVec3))
          (goto _label))))))

(event EventDestroyConversation
  (Variables|Default|SetWIllDestroy true)
  (bind _lerp (Timeline|ScaleUp Reverse)
    (:Update
      (Transformation|SetRelativeScale3D (Variables|Default|GetSM_Coin) (* _lerp (.Scale (Math|Transform|BreakTransform (Variables|Default|GetRelativeT))))))
    (:Finished
      (if (Variables|Default|GetWIllDestroy)
        (Actor|DestroyActor)))))

(fn ConstructionScript)

(fn RandomFloat
  (return (Math|Random|RandomFloatinRange -1.0 1.0)))