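; Interactable coin pickup that a kobold character collects by overlapping its box, provided it is not already holding a coin.
; On a one-time pickup it spawns a puff effect, destroys the rotating coin, snaps its hold component onto the kobold's coin attachment and reveals the held coin.
; It then flags the kobold as holding a coin, fires the CoinPickedUp dispatcher and plays audio.
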(event OnComponentBeginOverlap(Box)
  (params (OverlappedComponent :type Primitive%20Component%20Object%20Reference) (OtherActor :type Actor%20Object%20Reference) (OtherComp :type Primitive%20Component%20Object%20Reference) (OtherBodyIndex :type Integer) (bFromSweep :type Boolean) (SweepResult :type Hit%20Result%20Structure%20%28by%20ref%29))
  (bind _asbp_kobold_main (Utilities|Casting|CastToBP_KoboldMain OtherActor))
  (if (not (Variables|/Game/Blueprints/BP_KoboldMain.BP_KoboldMain_C|GetIsHoldingCoin _asbp_kobold_main))
    (Utilities|FlowControl|DoOnce false
      (:Completed
        (Niagara|SpawnSystematLocation "/Game/VFX/Puff_smaller_VFX.Puff_smaller_VFX" (Transformation|GetWorldLocation (Variables|/Game/Blueprints/BP_KoboldMain.BP_KoboldMain_C|GetCoinAttachment _asbp_kobold_main)))
        (Components|DestroyComponent (Variables|Default|GetRotatin_Coin))
        (Transformation|AttachComponentToComponent (Variables|Default|GetCoinHold) (Variables|/Game/Blueprints/BP_KoboldMain.BP_KoboldMain_C|GetCoinAttachment _asbp_kobold_main) "None" "SnapToTarget" "SnapToTarget" "KeepRelative" true)
        (Rendering|SetVisibility (Variables|Default|GetHeldCoin) true false)
        (Variables|/Game/Blueprints/BP_KoboldMain.BP_KoboldMain_C|SetIsHoldingCoin _asbp_kobold_main true)
        (Default|CallCoinPickedUp)
        (Audio|Components|Audio|Play (Variables|Default|GetAudio) 0.0)))))

(event EventBeginPlay)

(event Collision|EventActorBeginOverlap
  (params (OtherActor :type Actor%20Object%20Reference)))

(event EventTick
  (params (DeltaSeconds :type Float%20%28single-precision%29)))

(fn ConstructionScript)