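; Manages the stacked-kobold disguise, entrance door and detection countdown.
; Stack events update a counter that attaches or detaches the cape and hat and, before game start, opens or closes the door.
; A trigger box starts the game, camera follow and permanent door opening; stack events then toggle suspicion instead.
; Suspicion plays a reversible timeline that grows, shakes and reveals three exclamation marks at the kobolds' average height, calling game over when full.
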(event OnComponentBeginOverlap(StartSuspicionBoxColl)
  (params (OverlappedComponent :type Primitive%20Component%20Object%20Reference) (OtherActor :type Actor%20Object%20Reference) (OtherComp :type Primitive%20Component%20Object%20Reference) (OtherBodyIndex :type Integer) (bFromSweep :type Boolean) (SweepResult :type Hit%20Result%20Structure%20%28by%20ref%29))
  ;[1 0.4225 0.912] StartSuspition
  (Utilities|Casting|CastToBP_KoboldMain OtherActor)
  (Utilities|FlowControl|DoOnce false
    (:Completed
      (bind _outactors (Actor|GetAllActorsOfClass "/Game/ThirdPerson/Blueprints/BP_MainCamera.BP_MainCamera_C"))
      (Default|StartFollow (Utilities|Array|Get(acopy) _outactors))
      (Variables|Default|SetGameStarted true)
      (CallFunction|ExternalOpenDoor)
      (CallFunction|StopDoorWave))))

(event Custom|KoboldStacked
  (bind _result (Math|Integer|IncrementInt (Variables|Default|GetCounter))
    (:%20%20
      (if (>= _result 2)
        (|ActivateDisguise)
        (if (Variables|Default|GetGameStarted)
          ;[1 0.3102 0.9051] Suspicion
          (|SuspicionLogic) ; enters at Off
          (else
            ;[1 1 1] Door
            (|DoorHandler) ; enters at OpenCheck
          ))))))

(event Custom|KoboldUnstacked
  (bind _result (Math|Integer|DecrementInt (Variables|Default|GetCounter))
    (:%20%20
      (if (<= _result 2)
        (|DeactivateDisguise)
        (if (Variables|Default|GetGameStarted)
          ;[1 0.3102 0.9051] Suspicion
          (|SuspicionLogic)
          (else
            ;[1 1 1] Door
            (|DoorHandler) ; enters at Close
          ))))))

(event Custom|ExternalOpenDoor
  ;[1 1 1] Door
  (|DoorHandler))

(event EventBeginPlay
  (|UpdateValues)
  (Utilities|FlowControl|Sequence
    (:then_0
      (|DoorEffects))))

(fn ConstructionScript)

(fn CalculateKoboldAverage
  (params (Array :type Array%20of%20BP%20Kobold%20Main%20Object%20References))
  (bind _returnvalue (Game|Player|GetPlayerPawn 0))
  (bind _returnvalue_2 (Transformation|GetActorLocation _returnvalue))
  (Variables|Default|SetAverageKoboldX 0.0)
  (for _array_element Array
    (Variables|Default|SetAverageKoboldX (+ (.z (Transformation|GetActorLocation _array_element)) (Variables|Default|GetAverageKoboldX))))
  (return (Math|Vector|MakeVector (.x _returnvalue_2) (.y _returnvalue_2) (/ (Variables|Default|GetAverageKoboldX) (Utilities|Array|Length (Variables|Default|GetKoboldList))))))

(fn ExclamationRotation
  (params (Mark :type Scene%20Component%20Object%20Reference) (Lerp :type Float%20%28double-precision%29) (InTransform :type Transform%20%28by%20ref%29))
  (Transformation|SetRelativeRotation Mark (Math|Rotator|CombineRotators (.Rotation (Math|Transform|BreakTransform InTransform)) (Math|Rotator|MakeRotator 0.0 (* Lerp (Variables|Default|GetExclamationRotationMagnifier)) 0.0)) false false))

(fn SetExclamationScale
  (params (Alpha :type Float%20%28single-precision%29) (InTransform :type Transform%20%28by%20ref%29) (Target :type Scene%20Component%20Object%20Reference))
  (bind _scale (Math|Transform|BreakTransform InTransform))
  (Transformation|SetRelativeScale3D Target (Math|Vector|Lerp(Vector) _scale (* _scale 2.0) Alpha)))

(event Custom|StopDoorWave
  (bind _lerp (Timeline|WindyDoor Stop)
    (:Update
      (Transformation|SetRelativeRotation (Variables|Default|GetSM_Door) (Math|Rotator|CombineRotators (Variables|Default|GetDoorRelativeRotation) (Math|Rotator|MakeRotator 0.0 0.0 (* _lerp 7.0))) false false))
    (:Finished
      (if (not (Variables|Default|GetGameStarted))
        (Timeline|WindyDoor PlayFromStart)))))